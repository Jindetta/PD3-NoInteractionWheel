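; Mod actor that disables the circular interaction wheel by closing it without making a selection.
; On heist start it drops any cached wheel widget and enables Tick to search all widgets for the SBZCircularInteractionWidget.
; Tick binds to the widget's visibility changes, then switches itself off once a valid reference is held.
; A change to Visible or Hidden turns off select-on-close and deactivates the wheel.
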(event Custom|OnVisibilityChanged
  (params (InVisibility :type ESlateVisibility%20Enum :default "Visible"))
  (bind _interactionwidget (Variables|Default|GetInteractionWidget))
  (switch Utilities|FlowControl|Switch|SwitchonESlateVisibility InVisibility
    (:Visible
      _)
    (:Hidden
      _))
  (Variables|/Script/Starbreeze.SBZCircularInteractionWidget|SetbSelectOnClose _interactionwidget false)
  (Class|SBZCircularInteractionWidget|ActivateCircularWidget _interactionwidget false))

(event Custom|OnHeistStart
  (EventDispatchers|UnbindEventfromOnVisibilityChanged (Variables|Default|GetInteractionWidget) (EventDispatchers|CreateEvent :!event Custom|OnVisibilityChanged))
  (Variables|Default|SetInteractionWidget 0)
  (Actor|Tick|SetActorTickEnabled true))

(event EventBeginPlay
  (Actor|Tick|SetActorTickEnabled false)
  (bind _modloadermanagerinstance (CallFunction|GetModLoaderManager))
  (EventDispatchers|BindEventtoOnHeistStart _modloadermanagerinstance (EventDispatchers|CreateEvent :!event Custom|OnHeistStart)))

(event EventTick
  (params (DeltaSeconds :type Float%20%28single-precision%29))
  (Utilities|IsValid (Variables|Default|GetInteractionWidget)
    (:Is%20Valid
      (Actor|Tick|SetActorTickEnabled false))
    (:Is%20Not%20Valid
      (bind _foundwidgets (Widget|GetAllWidgetsOfClass "/Script/Starbreeze.SBZCircularInteractionWidget" false))
      (for _array_element _foundwidgets
        (bind _output_get (Variables|Default|SetInteractionWidget _array_element))
        (EventDispatchers|BindEventtoOnVisibilityChanged _output_get (EventDispatchers|CreateEvent :!event Custom|OnVisibilityChanged))))))

(fn ConstructionScript)